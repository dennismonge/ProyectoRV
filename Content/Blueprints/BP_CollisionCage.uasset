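; BP_CollisionCage is a target cage that registers when a BP_GrabbableBox lands inside it.
; An ActivateMoving event turns on side-to-side motion: Tick nudges the root along Y with very short MoveComponentTo calls, reversing when the Cube passes fixed world-space bounds.
; Tick also polls the Box's overlapping actors, and on finding a grabbable box sets Complete and respawns the referenced box.
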(event `MoveLeftRight`
  (bind _defaultsceneroot (`self.DefaultSceneRoot`))
  (bind _defaultsceneroot_2 (`self.DefaultSceneRoot`))
  (bind (_returnvalue_x _returnvalue_y) (`KismetMathLibrary.BreakVector` (`SceneComponent.K2_GetComponentLocation` (`self.Cube`))))
  (bind (_returnvalue_x_2 _returnvalue_y_2) (`KismetMathLibrary.BreakVector` (`SceneComponent.K2_GetComponentLocation` (`self.Cube`))))
  (bind (_relativelocation_x _relativelocation_y) (`KismetMathLibrary.BreakVector` (`SceneComponent.RelativeLocation` _defaultsceneroot)))
  (bind (_relativelocation_x_2 _relativelocation_y_2) (`KismetMathLibrary.BreakVector` (`SceneComponent.RelativeLocation` _defaultsceneroot_2)))
  ;[1 1 1] Hacemos que la CollisionCage se mueva de derecha a izquierda
  (if (`self.Right`)
    (`KismetSystemLibrary.MoveComponentTo` _defaultsceneroot (`KismetMathLibrary.MakeVector` 0.0 (+ _relativelocation_y 2.0)) (struct) false false 0.0001)
    (if (> _returnvalue_y_2 1300.0)
      (set `self.Right` false))
    (else
      (`KismetSystemLibrary.MoveComponentTo` _defaultsceneroot_2 (`KismetMathLibrary.MakeVector` 0.0 (- _relativelocation_y_2 2.0)) (struct) false false 0.0001)
      (if (< _returnvalue_y 1000.0)
        (set `self.Right` true)))))

(event `ActivateMoving`
  ;[1 1 1] Activamos el booleano del movimiento
  (set `self.Moving` true))

(event `self.ReceiveTick`
  (params (DeltaSeconds :type "Float (single-precision)"))
  ;[1 1 1] Si el booleano de Movimiento esta activo llamamos al evento 'MoveLeftRight', si no esta activo no hacemos nada
  (if (`self.Moving`)
    (`self.MoveLeftRight`))
  ;[1 1 1] Si dentro de la CollisionCage hay una GrabbableBox marcamos el booleano Completado a activo y Respawneamos la GrabbableBox
  (if (> (`KismetArrayLibrary.Array_Length` (`PrimitiveComponent.GetOverlappingActors` (`self.Box`) "/Game/Blueprints/BP_GrabbableBox.BP_GrabbableBox_C")) 0)
    (set `self.Complete` true)
    (`/Game/Blueprints/BP_GrabbableBox.Respawn` (`self.RefBP_GrabbableBox`))))

(fn `UserConstructionScript`)