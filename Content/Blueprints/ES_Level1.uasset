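; ES_Level1 is the Level 1 event system, guiding a three-target objective with a collision cage and point arrow.
; While active, Tick polls the cage's Complete flag, resets it and switches on a position counter, which the Construction Script increments initially.
; The first two completions move cage and overhead arrow to the next spawn and update dialogue progress.
; The third shows final text and deactivates the system.
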(event `self.ReceiveTick`
  (params (DeltaSeconds :type "Float (single-precision)"))
  (bind (_spawn2_x _spawn2_y _spawn2_z) (`KismetMathLibrary.BreakVector` (`self.Spawn2`)))
  (bind (_spawn3_x _spawn3_y _spawn3_z) (`KismetMathLibrary.BreakVector` (`self.Spawn3`)))
  (bind _rootcomponent (`Actor.RootComponent` (`self.RefBP_CollisionCage`)))
  ;[1 1 1] Comprobamos si el Event System Level 1 esta activo
  (if (`self.Active`)
    ;[1 1 1] Comprobamos si la CollisionCage esta Complete
    (if (== (`/Game/Blueprints/BP_CollisionCage.Complete` (`self.RefBP_CollisionCage`)) true)
      ;[1 1 1] Marcamos a false la variable Complete
      (set `/Game/Blueprints/BP_CollisionCage.Complete` false (`self.RefBP_CollisionCage`))
      ;[1 1 1] Dependiendo la el NumberPositionCage hacemos cosas distintas
      (switch `int` (`self.NumberPositionCage`)
        (:`1`
          ;[1 1 1] Movemos la CollisionCage a la siguiente posición  y aumentamos el NumberPositionCage
          (`KismetSystemLibrary.MoveComponentTo` _rootcomponent (`self.Spawn2`))
          (`KismetSystemLibrary.MoveComponentTo` (`Actor.RootComponent` (`self.RefBP_PointArrow`)) (`KismetMathLibrary.MakeVector` _spawn2_x _spawn2_y (+ _spawn2_z 160.0)))
          (`/Game/Blueprints/System_Dialogue.ChangeText` (`self.Ref_SystemDialogue`) "Target 1/3")
          (set `self.NumberPositionCage` (+ (`self.NumberPositionCage`) 1) :!label _label))
        (:`2`
          (`KismetSystemLibrary.MoveComponentTo` _rootcomponent (`self.Spawn3`))
          (`KismetSystemLibrary.MoveComponentTo` (`Actor.RootComponent` (`self.RefBP_PointArrow`)) (`KismetMathLibrary.MakeVector` _spawn3_x _spawn3_y (+ _spawn3_z 160.0)))
          (`/Game/Blueprints/System_Dialogue.ChangeText` (`self.Ref_SystemDialogue`) "Target 2/3")
          (goto _label))
        (:`3`
          ;[1 1 1] Añadimos un texto en partida y desactivamos el Event System Level 1
          (`/Game/Blueprints/System_Dialogue.FinalText` (`self.Ref_SystemDialogue`) "Target 3/3")
          (set `self.Active` false))))))

(fn `UserConstructionScript`
  ;[1 1 1] La posición de la caja será igual a 1
  (set `self.NumberPositionCage` (+ (`self.NumberPositionCage`) 1)))