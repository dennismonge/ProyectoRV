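; ES_Level2 is the event system for the second level, which drives the final zone of a reflex test.
; StartLevel teleports the player to the second zone, switches the GrabbableBox spawn and activates the system, while MoveCollisionCage relocates the cage and pointer arrow and starts the cage moving.
; While active, Tick polls the cage's Complete flag, resets it and shows the end-of-game message through the dialogue system.
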(event `Start Level`
  ;[1 1 1] Iniciamos el nivel 2, movemos al jugador a la segunda zona, cambiamos el Spawn de la GrabbableBox y activamos el Event System Level 2
  (`self.K2_TeleportTo` :`self` (`GameplayStatics.GetPlayerPawn` 0) :`DestLocation` (`self.SpawnPlayer`))
  (`/Game/Blueprints/BP_GrabbableBox.Change Spawn` (`self.RefBP_GrabbableBox`) 2)
  (set `self.Active` true))

(event `MoveCollisionCage`
  (bind (_spawncollisioncage_x _spawncollisioncage_y _spawncollisioncage_z) (`KismetMathLibrary.BreakVector` (`self.SpawnCollisionCage`)))
  ;[1 1 1] Movemos la CollisionCage y el PointArrow a la segunda zona. Luego activamos el movimiento de la CollisionCage
  (`self.K2_TeleportTo` :`self` (`self.RefBP_CollisionCage`) :`DestLocation` (`self.SpawnCollisionCage`))
  (`self.K2_TeleportTo` :`self` (`self.RefBP_PointArrow`) :`DestLocation` (`KismetMathLibrary.MakeVector` (- _spawncollisioncage_x 30.0) _spawncollisioncage_y (+ _spawncollisioncage_z 160.0)))
  (`/Game/Blueprints/BP_CollisionCage.ActivateMoving` (`self.RefBP_CollisionCage`)))

(event `self.ReceiveTick`
  (params (DeltaSeconds :type "Float (single-precision)"))
  ;[1 1 1] Comprobamos si el Event System Level 2 esta activo
  (if (`self.Active`)
    ;[1 1 1] Si la CollisionCage tiene el booleano Complete a true mostramos el mensaje de final de juego
    (if (== (`/Game/Blueprints/BP_CollisionCage.Complete` (`self.RefBP_CollisionCage`)) true)
      (set `/Game/Blueprints/BP_CollisionCage.Complete` false (`self.RefBP_CollisionCage`))
      (`/Game/Blueprints/System_Dialogue.FinalText` (`self.Ref_SystemDialogue`) "You've complet the Relfex Test, Congratulations!"))))

(fn `UserConstructionScript`)