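; BP_GrabbableBox is a physics box that can be sent back to one of two stored spawn locations.
; ChangeSpawn selects Spawn1 or Spawn2 as the active spawn, and the construction script defaults it to Spawn1.
; Respawn moves the static mesh to the active spawn and zeroes its linear velocity so it arrives without momentum.
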(event `Change Spawn`
  (params (NumberSpawn :type Integer))
  ;[1 1 1] Cambiamos el ActualSpawn  al número pasado por parámetro
  (switch `int` NumberSpawn
    (:`1`
      (set `self.ActualSpawn` (`self.Spawn1`)))
    (:`2`
      (set `self.ActualSpawn` (`self.Spawn2`)))))

(event `Respawn`
  ;[1 1 1] Spawneamos la GrabbableBox en su ActualSpawn con velocidad 0
  (`SceneComponent.K2_SetWorldLocation` (`self.StaticMesh`) (`self.ActualSpawn`) false false)
  (`PrimitiveComponent.SetPhysicsLinearVelocity` (`self.StaticMesh`) (0.0 0.0 0.0) false "None"))

(fn `UserConstructionScript`
  ;[1 1 1] Activamos el ActualSpawn al Spawn1
  (`self.Change Spawn` 1))