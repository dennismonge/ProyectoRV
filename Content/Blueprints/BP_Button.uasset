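; Pressure button that sinks while any actor overlaps its Box and rises back when clear, respawning a referenced grabbable box when pressed.
; Tick polls the overlaps and steps the mesh in Z through MoveComponentTo, clamped between zero and ButtonOffSet.
; Respawn is called on every overlapped tick that finds the mesh near the bottom.
; The construction script uses ButtonOffSet for both the Arrow length and the mesh's raised height.
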(event `self.ReceiveTick`
  (params (DeltaSeconds :type "Float (single-precision)"))
  (bind _staticmesh (`self.StaticMesh`))
  (bind _staticmesh_2 (`self.StaticMesh`))
  (bind (_relativelocation_x _relativelocation_y _relativelocation_z) (`KismetMathLibrary.BreakVector` (`SceneComponent.RelativeLocation` _staticmesh)))
  (bind (_relativelocation_x_2 _relativelocation_y_2 _relativelocation_z_2) (`KismetMathLibrary.BreakVector` (`SceneComponent.RelativeLocation` _staticmesh_2)))
  (bind (_relativelocation_x_3 _relativelocation_y_3 _relativelocation_z_3) (`KismetMathLibrary.BreakVector` (`SceneComponent.RelativeLocation` (`self.StaticMesh`))))
  ;[1 1 1] Comprobamos si hay algun Actor que este collisionando con nuestra Box
  (if (> (`KismetArrayLibrary.Array_Length` (`PrimitiveComponent.GetOverlappingActors` (`self.Box`) null)) 0)
    ;[1 1 1] Movemos el botón hacia abajo
    (`KismetSystemLibrary.MoveComponentTo` _staticmesh_2 (`KismetMathLibrary.MakeVector` 0.0 0.0 (`KismetMathLibrary.FClamp` (- _relativelocation_z_2 3.0) 0.0 (`self.ButtonOffSet`))) (struct) false false 0.0001)
    ;[1 1 1] Le decimos a la GrabbableBox que vuelva a Spawnear cuando consideremos que el botón ha sido pulsado
    (if (<= _relativelocation_z_3 2.0)
      (`/Game/Blueprints/BP_GrabbableBox.Respawn` (`self.RefBP_GrabbableBox`)))
    (else
      ;[1 1 1] Movemos el botón hacia arriba
      (`KismetSystemLibrary.MoveComponentTo` _staticmesh (`KismetMathLibrary.MakeVector` 0.0 0.0 (`KismetMathLibrary.FClamp` (+ _relativelocation_z 3.0) 0.0 (`self.ButtonOffSet`))) (struct) false false 0.0001))))

(fn `UserConstructionScript`
  (bind _buttonoffset (`self.ButtonOffSet`))
  ;[1 1 1] Asignamos la longitud original del 'Arrow' y movemos la caja en Z hasta esa posición
  (set `ArrowComponent.ArrowLength` _buttonoffset (`self.Arrow`))
  (`SceneComponent.K2_SetRelativeLocation` (`self.StaticMesh`) (`KismetMathLibrary.MakeVector` 0.0 0.0 _buttonoffset) false false))