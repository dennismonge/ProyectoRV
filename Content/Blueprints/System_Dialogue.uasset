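; Dialogue system that shows timed on-screen text for levels 1 and 2 through TextRender actors.
; A tick-counted countdown, so frame-rate dependent, advances a line index that switches between preset texts.
; ChangeText shows temporary text, while FinalText leads into the closing line and then starts level 2 through RefESLevel2.
; Level 2's last step repeatedly calls MoveCollisionCage and blanks the first text actor rather than its own.
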(event `FinalText`
  (params (NewText :type Text))
  ;[1 1 1] Ativamos un texto final
  (`TextRenderComponent.K2_SetText` (`TextRenderActor.TextRender` (`self.Ref_TextRenderActor`)) NewText)
  (set `self.Time_Text` (`self.Time_Text_Screen`))
  (set `self.LineText` 3))

(event `ChangeText`
  (params (New_Text :type Text))
  ;[1 1 1] Mostramos un texto que desaparecra pasado un tiempo
  (`TextRenderComponent.K2_SetText` (`TextRenderActor.TextRender` (`self.Ref_TextRenderActor`)) New_Text)
  (set `self.Time_Text` (`self.Time_Text_Screen`))
  (set `self.LineText` 2))

(event `self.ReceiveTick`
  (params (DeltaSeconds :type "Float (single-precision)"))
  ;[1 1 1] Reducimos de 1 en 1 el valor de TimeText hasta que sea 0
  (set `self.Time_Text` (- (`self.Time_Text`) 1))
  (if (== (`self.Time_Text`) 0)
    (set `self.Time_Text` (`self.Time_Text_Screen`))
    ;[1 1 1] Dependiendo del nivel en el que estamos apareceran unos textos u otros
    (if (== (`self.Level`) 1)
      ;[1 1 1] Textos en Pantalla del nivel 1
      (switch `int` (`self.LineText`)
        (:`0`
          (`TextRenderComponent.K2_SetText` (`TextRenderActor.TextRender` (`self.Ref_TextRenderActor`)) (`self.Text2`))
          (set `self.LineText` (+ (`self.LineText`) 1)))
        (:`1`
          (`TextRenderComponent.K2_SetText` (`TextRenderActor.TextRender` (`self.Ref_TextRenderActor`)) (`self.Text3`))
          (set `self.LineText` (+ (`self.LineText`) 1)))
        (:`2`
          (`TextRenderComponent.K2_SetText` (`TextRenderActor.TextRender` (`self.Ref_TextRenderActor`)) (`self.TextBlank`)))
        (:`3`
          (`TextRenderComponent.K2_SetText` (`TextRenderActor.TextRender` (`self.Ref_TextRenderActor`)) (`self.Text_Final`))
          (set `self.LineText` 4))
        (:`4`
          (set `self.Level` 2)
          (set `self.LineText` 0)
          (`/Game/Blueprints/ES_Level2.Start Level` (`self.RefES_Level2`))))
      (elif (== (`self.Level`) 2)
        ;[1 1 1] Textos en pantalla del nivel 2
        (switch `int` (`self.LineText`)
          (:`0`
            (`TextRenderComponent.K2_SetText` (`TextRenderActor.TextRender` (`self.Ref_TextRenderActor2`)) (`self.Text2_2`))
            (set `self.LineText` (+ (`self.LineText`) 1)))
          (:`1`
            (`TextRenderComponent.K2_SetText` (`TextRenderActor.TextRender` (`self.Ref_TextRenderActor2`)) (`self.Text3_2`))
            (set `self.LineText` (+ (`self.LineText`) 1)))
          (:`2`
            (`TextRenderComponent.K2_SetText` (`TextRenderActor.TextRender` (`self.Ref_TextRenderActor`)) (`self.TextBlank`))
            (`/Game/Blueprints/ES_Level2.MoveCollisionCage` (`self.RefES_Level2`))))))))

(fn `UserConstructionScript`
  ;[1 1 1] Seteamos el tiempo que dura el texto en pantalla
  (set `self.Time_Text` (`self.Time_Text_Screen`)))